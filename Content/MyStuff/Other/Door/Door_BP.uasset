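; Interactable sliding door that can be locked, with a point light showing red when locked and green when unlocked.
; Interaction opens it if unlocked; a required key is checked through the player's inventory component and unlocks it first.
; A linked trigger unlocks keyless doors when on, and locks and closes the door when off.
; A timeline slides the cube along DoorsDirection and reverses when the player's overlap ends.
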(event OnTriggered(Trigger)
  (params (IsTriggered :type Boolean))
  ;[0.15 0.1359 0.1361 0.5] When Overlapping with button
  (if IsTriggered
    (Variables|Default|Getrequire%20Key
      (:then)
      (:else
        (CallFunction|UnlockDoor)))
    (else
      (CallFunction|LockDoor))))

(event Custom|OpenDoor
  ;[1 0 0.0426 0.009] Movement
  ;;[0.15 0.05547 0.05547 0.5] IsLock Sequence
  (if (not (Variables|Default|GetLocked))
    (bind _position (Timeline|DoorOpen Play)
      (:Update
        (Transformation|SetRelativeLocation (Variables|Default|GetCube) (* (Variables|Default|GetDoors%20Direction) _position) false false)))))

(event Custom|CloseDoor
  ;[1 0 0.0426 0.009] Movement
  (bind _position (Timeline|DoorOpen Reverse)
    (:Update
      (Transformation|SetRelativeLocation (Variables|Default|GetCube) (* (Variables|Default|GetDoors%20Direction) _position) false false))))

(event EventBeginPlay)

(event EventInteractwith
  (params (PlayerCharacter :type BP%20First%20Person%20Character%20Object%20Reference))
  (bind _require_key (Variables|Default|Getrequire%20Key)
    (:then
      (bind _return_success (Default|InventoryList (Variables|/Game/FirstPerson/Blueprints/BP_FirstPersonCharacter.BP_FirstPersonCharacter_C|GetBP_Inventiry_System PlayerCharacter) _require_key 1))
      (if _return_success
        (CallFunction|UnlockDoor)
        (CallFunction|OpenDoor :!label _label)))
    (:else
      (goto _label))))

(event EventTick
  (params (DeltaSeconds :type Float%20%28single-precision%29)))

(event Collision|EventActorBeginOverlap
  (params (OtherActor :type Actor%20Object%20Reference))
  ;[0.15 0.15 0.15 0.5] WHen Overlapping with Door
)

(event Collision|EventActorEndOverlap
  (params (OtherActor :type Actor%20Object%20Reference))
  ;[0.15 0.15 0.15 0.5] WHen Overlapping with Door
  (if (== OtherActor (Game|GetPlayerCharacter 0))
    (CallFunction|CloseDoor)))

(fn ConstructionScript
  (Rendering|Components|Light|SetLightColor (Variables|Default|GetPointLight) (Math|Color|SelectColor "(R=1.000000,G=0.000000,B=0.000000,A=1.000000)" "(R=0.234243,G=1.000000,B=0.000000,A=1.000000)" (Variables|Default|GetLocked)) true))

(fn UnlockDoor
  (bind _output_get (Variables|Default|SetLocked false))
  ;[0.15 0.15 0.15 0.5] Color Change
  (Rendering|Components|Light|SetLightColor (Variables|Default|GetPointLight) (Math|Color|SelectColor "(R=1.000000,G=0.000000,B=0.000000,A=1.000000)" "(R=0.234243,G=1.000000,B=0.000000,A=1.000000)" _output_get) true)
  (Variables|Default|Getrequire%20Key
    (:then
      (if (Variables|Default|GetDestroy%20Key%20on%20Unlock)
        (Variables|Default|Setrequire%20Key 0)))
    (:else)))

(fn LockDoor
  (bind _output_get (Variables|Default|SetLocked true))
  ;[0.15 0.15 0.15 0.5] Color Change
  (Rendering|Components|Light|SetLightColor (Variables|Default|GetPointLight) (Math|Color|SelectColor "(R=1.000000,G=0.000000,B=0.000000,A=1.000000)" "(R=0.234243,G=1.000000,B=0.000000,A=1.000000)" _output_get) true)
  ;[0.15 0.15 0.15 0.5] Making Door Close When Locked
  (CallFunction|CloseDoor))

(fn Lookat
  (return "open" "Door"))