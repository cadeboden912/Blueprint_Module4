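; BP_PressurePad is a pressure pad in the door folder that reacts only to the player character overlapping it.
; Stepping on lowers the Cube mesh and fires the OnTriggered dispatcher with true, so other actors can respond.
; Stepping off raises the Cube and starts a timer of configurable Time, apparently bound to Timeout, which broadcasts false.
; Re-entry does not clear a running timer.
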(event Custom|ButtonTrigger
  ;[0.15 0.15 0.15 0.5] Calling Event Dispatch
  (Default|CallOnTriggered true)
  (Transformation|SetRelativeLocation (Variables|Default|GetCube) "0.000000,0.000000,-6.000000" false false))

(event Custom|ButtonUntriggered
  ;[0.15 0.15 0.15 0.5] SettingTimer and button Location change
  (Transformation|SetRelativeLocation (Variables|Default|GetCube) "0, 0, 0" false false)
  (Utilities|Time|SetTimerbyEvent (EventDispatchers|CreateEvent :!event Timeout) (Variables|Default|GetTime)))

(event Collision|EventActorBeginOverlap
  (params (OtherActor :type Actor%20Object%20Reference))
  (if (== OtherActor (Game|GetPlayerCharacter 0))
    (CallFunction|ButtonTrigger)))

(event Collision|EventActorEndOverlap
  (params (OtherActor :type Actor%20Object%20Reference))
  (if (== OtherActor (Game|GetPlayerCharacter 0))
    (CallFunction|ButtonUntriggered)))

(fn ConstructionScript)

(fn Timeout
  (Default|CallOnTriggered false))