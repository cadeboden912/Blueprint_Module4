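; Lever actor that the player can pull to toggle between on and off, reporting "Pull" and "Lever" as its look-at text.
; Interactwith plays or reverses the Position timeline based on IsActive, rotating the Scene component through 90 degrees.
; When the timeline finishes, its direction sets IsActive and is broadcast through OnTriggered, so the state changes only at the end of the swing.
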(event EventBeginPlay
  (|CallParentFunction) ; This node is disabled and will not be called.\nDrag off pins to build functionality.
)

(event Collision|EventActorBeginOverlap
  (params (OtherActor :type Actor%20Object%20Reference))
  (|CallParentFunction OtherActor) ; This node is disabled and will not be called.\nDrag off pins to build functionality.
)

(event EventTick
  (params (DeltaSeconds :type Float%20%28single-precision%29))
  (|CallParentFunction DeltaSeconds) ; This node is disabled and will not be called.\nDrag off pins to build functionality.
)

(event EventInteractwith
  (params (PlayerCharacter :type BP%20First%20Person%20Character%20Object%20Reference))
  (if (Variables|Default|GetIsActive)
    (bind (_direction _newtrack_0) (Timeline|Position Reverse)
      (:Update
        (Transformation|SetRelativeRotation (Variables|Default|GetScene) (Math|Rotator|Lerp(Rotator) "0, 0, 0" "90.000000,0.000000,0.000000" _newtrack_0) false false))
      (:Finished
        (Default|CallOnTriggered (Utilities|Select :Index _direction :Forward true :Backward false))
        (Variables|Default|SetIsActive (Utilities|Select :Index _direction :Forward true :Backward false))))
    (else
      (Timeline|Position Play))))

(fn ConstructionScript
  (|CallParentFunction))

(fn Lookat
  (return "Pull" "Lever"))