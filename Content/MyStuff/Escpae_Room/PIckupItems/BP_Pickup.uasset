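; BP_Pickup is a data-driven pickup actor that the player can interact with to collect an item.
; Its construction script applies the static mesh from its item DataAsset.
; Interactwith adds the item and quantity to the player's inventory component, destroying the actor only if that succeeds and the asset flags destruction on pickup.
; Look At returns a "pickup" verb with the DataAsset converted to text as the noun.
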(event EventBeginPlay)

(event Collision|EventActorBeginOverlap
  (params (OtherActor :type Actor%20Object%20Reference)))

(event EventTick
  (params (DeltaSeconds :type Float%20%28single-precision%29)))

(event EventInteractwith
  (params (PlayerCharacter :type BP%20First%20Person%20Character%20Object%20Reference))
  (bind _dataasset (Variables|Default|GetDataAsset))
  (bind _return_success (Default|AddtoInventory (Variables|/Game/FirstPerson/Blueprints/BP_FirstPersonCharacter.BP_FirstPersonCharacter_C|GetBP_Inventiry_System PlayerCharacter) _dataasset (Variables|Default|GetQuantity)))
  (if (and _return_success (Variables|/Game/MyStuff/Escpae_Room/PIckupItems/Data_As/DA_Item.DA_Item_C|GetIsdestroyedonPickup _dataasset))
    (Actor|DestroyActor)))

(fn ConstructionScript
  (bind _dataasset (Variables|Default|GetDataAsset)
    (:then
      (Components|StaticMesh|SetStaticMesh (Variables|Default|GetStaticMesh) (Variables|/Game/MyStuff/Escpae_Room/PIckupItems/Data_As/DA_Item.DA_Item_C|GetStatic%20Mesh _dataasset)))
    (:else)))

(fn Lookat
  (return "pickup" (Utilities|Text|ToText(Object) (Variables|Default|GetDataAsset))))