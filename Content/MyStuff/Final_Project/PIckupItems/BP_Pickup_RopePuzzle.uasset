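; BP_Pickup_RopePuzzle is an interactable pickup tied to a bottle-placement puzzle.
; Each valid all-bottles-placed event decrements BottlesPlaced; at zero, ItemFall enables physics on the BurlapSack and prints a debug message.
; When not Locked, interaction adds the DataAsset item to the player's inventory, destroying the actor if the asset flags it.
; LookAt supplies pickup prompt text; the construction script's mesh setup is disconnected.
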(event Custom|AllBottlesPlacedValid_Event
  ;[0.15 0.15 0.15 0.5] Check for Bottles Placed
  (bind _result (Math|Integer|DecrementInt (Variables|Default|GetBottlesPlaced))
    (:%20%20
      (if (== _result 0)
        (CallFunction|ItemFall)))))

(event Custom|ItemFall
  ;[0.15 0.15 0.15 0.5] Upon all bottles Placed
  (if true
    (Physics|SetSimulatePhysics (Variables|Default|Getburlap_sack) true)
    (Development|PrintString "Hello")))

(event EventBeginPlay
  ;[0.15 0.15 0.15 0.5] Check for Bottles Placed
  (EventDispatchers|BindEventtoAllBottlesPlacedValid (delegate Custom|AllBottlesPlacedValid_Event)))

(event EventInteractwith
  (params (PlayerCharacter :type BP%20First%20Person%20Character%20Object%20Reference))
  (bind _dataasset (Variables|Default|GetDataAsset))
  ;[0.15 0.15 0.15 0.5] Upon all bottles Placed
  ;;[0.15 0.15 0.15 0.5] Interact
  (if (not (Variables|Default|GetLocked))
    (bind _return_success (Default|AddtoInventory (Variables|/Game/FirstPerson/Blueprints/BP_FirstPersonCharacter.BP_FirstPersonCharacter_C|GetBP_Inventiry_System PlayerCharacter) _dataasset (Variables|Default|GetQuantity)))
    (if (and _return_success (Variables|/Game/MyStuff/Final_Project/PIckupItems/Data_As/DA_Item.DA_Item_C|GetIsdestroyedonPickup _dataasset))
      (Actor|DestroyActor))))

(fn ConstructionScript)

(fn Lookat
  (return "pickup" (Utilities|Text|ToText(Object) (Variables|Default|GetDataAsset))))