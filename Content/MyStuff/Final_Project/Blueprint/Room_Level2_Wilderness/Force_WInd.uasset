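; Toggleable wind volume in the Level 2 Wilderness room that lifts the first-person player.
; Activated flips the wind flag and plays or reverses a timeline that adds yaw to a cube, while a looping timer adds only zero rotation.
; Entering the capsule with wind on inverts the character's gravity, sets upward velocity and adds a downward force.
; Leaving the capsule restores normal gravity.
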(event OnComponentBeginOverlap(Capsule)
  (params (OverlappedComponent :type Primitive%20Component%20Object%20Reference) (OtherActor :type Actor%20Object%20Reference) (OtherComp :type Primitive%20Component%20Object%20Reference) (OtherBodyIndex :type Integer) (bFromSweep :type Boolean) (SweepResult :type Hit%20Result%20Structure%20%28by%20ref%29))
  ;[0.15 0.15 0.15 0.5] Overlap
  (if (Variables|Default|GetWindOIn)
    (bind _asbp_first_person_character (Utilities|Casting|CastToBP_FirstPersonCharacter OtherActor))
    (Variables|/Script/Engine.CharacterMovementComponent|SetGravityScale (Variables|/Script/Engine.Character|GetCharacterMovement _asbp_first_person_character) -1.0)
    (Variables|/Script/Engine.MovementComponent|SetVelocity (Variables|/Script/Engine.Character|GetCharacterMovement _asbp_first_person_character) (Math|Vector|MakeVector 0.0 0.0 1e+02))
    (Physics|AddForce (Variables|/Script/Engine.Character|GetCharacterMovement _asbp_first_person_character) "0.000000,0.000000,-100.000000")))

(event OnComponentEndOverlap(Capsule)
  (params (OverlappedComponent :type Primitive%20Component%20Object%20Reference) (OtherActor :type Actor%20Object%20Reference) (OtherComp :type Primitive%20Component%20Object%20Reference) (OtherBodyIndex :type Integer))
  ;[0.15 0.15 0.15 0.5] Leav Overlap
  (bind _asbp_first_person_character (Utilities|Casting|CastToBP_FirstPersonCharacter OtherActor))
  (Variables|/Script/Engine.CharacterMovementComponent|SetGravityScale (Variables|/Script/Engine.Character|GetCharacterMovement _asbp_first_person_character) 1.0))

(event Custom|Activated
  ;[0.15 0.15 0.15 0.5] Animation
  (if (Variables|Default|GetWindOIn)
    (Variables|Default|SetWindOIn false)
    (bind _newtrack_0 (Timeline|WIndEffect Reverse)
      (:Update
        (Transformation|AddRelativeRotation (Variables|Default|GetCube) (Math|Rotator|MakeRotator 0.0 0.0 (Math|Float|Lerp 0.0 22.5 _newtrack_0)) false false)
        (if (not (Variables|Default|GetWindOIn))
          (Utilities|Time|PauseTimerbyHandle (stale _returnvalue))
          (else
            (bind _returnvalue (Utilities|Time|SetTimerbyEvent (delegate Custom|Turn%20on) (Utilities|Time|GetWorldDeltaSeconds) true))))))
    (else
      (Variables|Default|SetWindOIn true)
      (Timeline|WIndEffect Play))))

(event Custom|Turn%20on
  ;[0.15 0.15 0.15 0.5] Animation
  (Transformation|AddRelativeRotation (Variables|Default|GetCube) "0, 0, 0" false false))

(fn ConstructionScript)