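; Final door for the Level 2 wilderness room that slides open once the lantern puzzle is complete.
; On BeginPlay it binds to the AllLanternsLit event, and each firing decrements a Quantity counter.
; When the counter reaches zero, a timeline moves the FinalDoor component's relative location by scaling an offset vector with its track value.
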(event Custom|AllLanternsLit_Event
  (bind _result (Math|Integer|DecrementInt (Variables|Default|GetQuantity))
    (:%20%20
      (if (== _result 0)
        (CallFunction|DoorOpen)))))

(event Custom|Door%20Open
  (bind _newtrack_0 (Timeline|Dopenanime Play)
    (:Update
      (Transformation|SetRelativeLocation (Variables|Default|GetFinalDoor) (* _newtrack_0 (Variables|Default|GetNewLoc)) false false))))

(event EventBeginPlay
  (EventDispatchers|BindEventtoAllLanternsLit (delegate Custom|AllLanternsLit_Event)))

(fn ConstructionScript)