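; Relic pedestal for the Level 2 Wilderness room, where the player places a required inventory item.
; On interact, it checks the player's inventory, removes one item, then once only shows the item's mesh, switches the cube to its On material and spins the relic via a timeline.
; Look At builds a "Placed" or "requires" prompt from the same inventory check.
; The all-relics-placed call and tested relic removal are disconnected.
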(event EventInteractwith
  (params (PlayerCharacter :type BP%20First%20Person%20Character%20Object%20Reference))
  (bind _bp_inventiry_system (Variables|/Game/FirstPerson/Blueprints/BP_FirstPersonCharacter.BP_FirstPersonCharacter_C|GetBP_Inventiry_System PlayerCharacter))
  (bind _item (Variables|Default|Getitem)
    (:then
      (bind _return_success (Default|InventoryList _bp_inventiry_system _item (Variables|Default|GetQuanitity)))
      (if _return_success
        (Default|RemovefromInventory _bp_inventiry_system _item 1)
        (Utilities|FlowControl|DoOnce false
          (:Completed
            (Components|StaticMesh|SetStaticMesh (Variables|Default|Getrelic) (Variables|/Game/MyStuff/Final_Project/PIckupItems/Data_As/DA_Item.DA_Item_C|GetStatic%20Mesh (Variables|Default|Getitem)))
            (Rendering|Material|SetMaterial (Variables|Default|GetCube) 0 "/Game/MyStuff/Other/Elevator_Components/On.On")
            ;[0.15 0.15 0.15 0.5] Rotate object
            (bind _newtrack_0 (Timeline|Rotating%20relic Play)
              (:Update
                (Transformation|AddRelativeRotation (Variables|Default|Getrelic) (Math|Rotator|MakeRotator 0.0 0.0 (Math|Float|Lerp 0.0 22.5 _newtrack_0)) false false)))))))
    (:else)))

(fn ConstructionScript)

(fn Lookat
  (bind _return_success (Default|InventoryList (Actor|GetComponentbyClass (Game|GetPlayerCharacter 0) "/Game/MyStuff/Final_Project/PIckupItems/Data_As/Inventory/BP_Inventory_System.BP_Inventory_System_C") (Variables|Default|Getitem) 1))
  (if _return_success
    (return "Placed" (Variables|/Game/MyStuff/Final_Project/PIckupItems/Data_As/DA_Item.DA_Item_C|GetName (Variables|Default|Getitem)))
    (else
      (return "requires" (Variables|/Game/MyStuff/Final_Project/PIckupItems/Data_As/DA_Item.DA_Item_C|GetName (Variables|Default|Getitem))))))