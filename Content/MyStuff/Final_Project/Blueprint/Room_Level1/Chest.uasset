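; Interactable chest for a level-one room that prompts "Modify Chest Code" when looked at.
; Interacting toggles a passcode widget on screen, switching input mode and mouse cursor on and off through a FlipFlop.
; A separate ChestOpen event plays a timeline that moves the chest's cube by updating its relative location.
; An older widget toggle graph is left unconnected and never runs.
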(event Custom|ChestOpen
  (bind _newtrack_0 (Timeline|Timeline Play)
    (:Update
      (Transformation|SetRelativeLocation (Variables|Default|GetCube) (+ _newtrack_0 (Variables|Default|GetNew%20Location)) false false))))

(event EventInteractwith
  (params (PlayerCharacter :type BP%20First%20Person%20Character%20Object%20Reference))
  (bind _returnvalue (Game|GetPlayerController 0))
  (Utilities|FlowControl|FlipFlop
    (:A
      (bind _returnvalue_2 (UserInterface|CreateWidget "/Game/MyStuff/Final_Project/Widgets/ChestPasscode.ChestPasscode_C"))
      (UserInterface|Viewport|AddtoViewport _returnvalue_2 0)
      (Input|SetInputModeGameandUI _returnvalue 0 "DoNotLock" true false)
      (Variables|/Script/Engine.PlayerController|SetbShowMouseCursor _returnvalue true))
    (:B
      (bind _foundwidgets (Widget|GetAllWidgetsOfClass "/Game/MyStuff/Final_Project/Widgets/ChestPasscode.ChestPasscode_C" true))
      (Widget|RemovefromParent _foundwidgets)
      (Input|SetInputModeGameOnly _returnvalue true)
      (Variables|/Script/Engine.PlayerController|SetbShowMouseCursor _returnvalue false))))

(fn ConstructionScript)

(fn Lookat
  (return "Modify" "Chest Code"))