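; PaintingPuzzle is an interactable item slot for a Level 1 puzzle that accepts a required inventory item.
; On interact, it checks the player's inventory, removes the stocked amount of the item and shows its mesh on the placement component.
; If a connected light is valid, it turns green and CallSettingtTowerPieces is called.
; Look At returns an "Inserted" or "Requires" prompt with the item name, based on current inventory.
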(event EventBeginPlay
  (|CallParentFunction) ; This node is disabled and will not be called.\nDrag off pins to build functionality.
)

(event Collision|EventActorBeginOverlap
  (params (OtherActor :type Actor%20Object%20Reference))
  (|CallParentFunction OtherActor) ; This node is disabled and will not be called.\nDrag off pins to build functionality.
)

(event EventTick
  (params (DeltaSeconds :type Float%20%28single-precision%29))
  (|CallParentFunction DeltaSeconds) ; This node is disabled and will not be called.\nDrag off pins to build functionality.
)

(event EventInteractwith
  (params (PlayerCharacter :type BP%20First%20Person%20Character%20Object%20Reference))
  (bind _bp_inventiry_system (Variables|/Game/FirstPerson/Blueprints/BP_FirstPersonCharacter.BP_FirstPersonCharacter_C|GetBP_Inventiry_System PlayerCharacter))
  (bind _item (Variables|Default|GetItem))
  (bind _connected_light (Variables|Default|GetConnected%20Light))
  (Variables|Default|GetItem
    (:then
      (bind (_return_success _instock) (Default|InventoryList _bp_inventiry_system _item 1))
      (if _return_success
        (Default|RemovefromInventory _bp_inventiry_system _item _instock)
        (Components|StaticMesh|SetStaticMesh (Variables|Default|GetTowerPlacemen%20t) (Variables|/Game/MyStuff/Final_Project/PIckupItems/Data_As/DA_Item.DA_Item_C|GetStatic%20Mesh (Variables|Default|GetItem)))
        (Utilities|IsValid _connected_light
          (:Is%20Valid
            (Rendering|Components|Light|SetLightColor (Variables|/Game/MyStuff/Final_Project/Blueprint/Room_Level1/Rm_1_Lights.Rm_1_Lights_C|GetPointLight _connected_light) "(R=0.000000,G=1.000000,B=0.028727,A=1.000000)" true)
            (Default|CallSettingtTowerPieces)))))
    (:else)))

(fn ConstructionScript
  (|CallParentFunction))

(fn Lookat
  (bind _return_success (Default|InventoryList (Actor|GetComponentbyClass (Game|GetPlayerCharacter 0) "/Game/MyStuff/Final_Project/PIckupItems/Data_As/Inventory/BP_Inventory_System.BP_Inventory_System_C") (Variables|Default|GetItem) 1))
  (if _return_success
    (return "Inserted " (Variables|/Game/MyStuff/Final_Project/PIckupItems/Data_As/DA_Item.DA_Item_C|GetName (Variables|Default|GetItem)))
    (else
      (return "Requires" (Variables|/Game/MyStuff/Final_Project/PIckupItems/Data_As/DA_Item.DA_Item_C|GetName (Variables|Default|GetItem))))))