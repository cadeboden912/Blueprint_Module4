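; Interactable journal actor for a Level 1 room that the player can open and close to read.
; Each Interactwith event flips between showing the OldM_Journal widget with the mouse cursor and a paper sound, and removing that widget and hiding the cursor.
; Closing finds the open widget by class rather than keeping a reference.
; A LookAt function supplies the "found" verb and "Journal" noun.
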(event EventBeginPlay)

(event Collision|EventActorBeginOverlap
  (params (OtherActor :type Actor%20Object%20Reference)))

(event EventTick
  (params (DeltaSeconds :type Float%20%28single-precision%29)))

(event EventInteractwith
  (params (PlayerCharacter :type BP%20First%20Person%20Character%20Object%20Reference))
  (bind _returnvalue (Game|GetPlayerController 0))
  (Utilities|FlowControl|FlipFlop
    (:A
      (Variables|/Script/Engine.PlayerController|SetbShowMouseCursor _returnvalue true)
      (bind _returnvalue_2 (UserInterface|CreateWidget "/Game/MyStuff/Final_Project/Widgets/OldM_Journal.OldM_Journal_C"))
      (UserInterface|Viewport|AddtoViewport _returnvalue_2 0)
      (Audio|PlaySound2D "/Game/MyStuff/Final_Project/Audio/Book_Note_Paper.Book_Note_Paper" 1.0 1.0 0.0 0 0))
    (:B
      (bind _foundwidgets (Widget|GetAllWidgetsOfClass "/Game/MyStuff/Final_Project/Widgets/OldM_Journal.OldM_Journal_C" true))
      (Widget|RemovefromParent _foundwidgets)
      (Variables|/Script/Engine.PlayerController|SetbShowMouseCursor _returnvalue false))))

(fn ConstructionScript)

(fn Lookat
  (return "found" "Journal"))