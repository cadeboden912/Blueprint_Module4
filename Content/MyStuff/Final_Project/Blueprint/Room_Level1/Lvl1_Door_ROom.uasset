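; A Level 1 room door that unlocks and opens by itself once the required tower pieces are in.
; It binds to a tower-pieces event on BeginPlay and decrements a counter each time it fires, unlocking and opening after a short delay at zero.
; Opening uses a timeline to move the Scene component, calling the door sound on every update.
; Look-at returns prompt text, but the interact event is empty.
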(event Custom|Open%20DoorFloor1_Room
  ;[0.15 0.15 0.15 0.5] Door
  (if (not (Variables|Default|GetLocked))
    (bind _opendoor (Timeline|Timeline Play)
      (:Update
        (Transformation|SetRelativeLocation (Variables|Default|GetScene) (* (Variables|Default|GetNew%20Location) _opendoor) false false)
        (Audio|PlaySound2D "/Game/MyStuff/Final_Project/Audio/Door.Door" 1.0 1.0 0.0 0 0)))))

(event Custom|AllTowerPiecesIn_Event
  ;[0.15 0.15 0.15 0.5] TowerPieces Needed
  (bind _result (Math|Integer|DecrementInt (Variables|Default|GetTowerpieces))
    (:%20%20
      (if (== _result 0)
        (CallFunction|UnlockDoor)
        (Utilities|FlowControl|Delay 1.5)
        (CallFunction|OpenDoorFloor1Room)))))

(event EventBeginPlay
  ;[0.15 0.15 0.15 0.5] TowerPieces Needed
  (EventDispatchers|BindEventtoAllTowerPiecesin (delegate Custom|AllTowerPiecesIn_Event)))

(event EventInteractwith
  (params (PlayerCharacter :type BP%20First%20Person%20Character%20Object%20Reference)))

(event EventTick
  (params (DeltaSeconds :type Float%20%28single-precision%29)))

(fn ConstructionScript)

(fn LockDoor
  (Variables|Default|SetLocked true))

(fn UnlockDoor
  (Variables|Default|SetLocked false))

(fn Lookat
  (return "Opens" "Door"))