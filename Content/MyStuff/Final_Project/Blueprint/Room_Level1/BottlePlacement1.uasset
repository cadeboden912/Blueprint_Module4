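; Interactable bottle placement spot, apparently for the Level 1 room, that takes a required item from the player's inventory.
; On interact, it checks the inventory component for the item, calls its removal, then once only shows the item's mesh, plays a sound and calls the AreBottlesPlaced dispatcher.
; Look At returns a "Place" or "Requires" prompt with the item name, depending on whether the player holds it.
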(event EventBeginPlay
  (|CallParentFunction) ; This node is disabled and will not be called.\nDrag off pins to build functionality.
)

(event Collision|EventActorBeginOverlap
  (params (OtherActor :type Actor%20Object%20Reference))
  (|CallParentFunction OtherActor) ; This node is disabled and will not be called.\nDrag off pins to build functionality.
)

(event EventTick
  (params (DeltaSeconds :type Float%20%28single-precision%29))
  (|CallParentFunction DeltaSeconds) ; This node is disabled and will not be called.\nDrag off pins to build functionality.
)

(event EventInteractwith
  (params (PlayerCharacter :type BP%20First%20Person%20Character%20Object%20Reference))
  (bind _bp_inventiry_system (Variables|/Game/FirstPerson/Blueprints/BP_FirstPersonCharacter.BP_FirstPersonCharacter_C|GetBP_Inventiry_System PlayerCharacter))
  (bind _item (Variables|Default|Getitem))
  (bind _item_2 (Variables|Default|Getitem)
    (:then
      (bind _return_success (Default|InventoryList _bp_inventiry_system _item_2 (Variables|Default|GetQuantity)))
      (if _return_success
        (Default|RemovefromInventory _bp_inventiry_system _item)
        (Utilities|FlowControl|DoOnce false
          (:Completed
            (Components|StaticMesh|SetStaticMesh (Variables|Default|GetStaticMesh) (Variables|/Game/MyStuff/Final_Project/PIckupItems/Data_As/DA_Item.DA_Item_C|GetStatic%20Mesh _item))
            (Audio|PlaySound2D (Variables|Default|Getsound) 1.0 1.0 0.0 0 0)
            (Default|CallAreBottlesPlaced)))))
    (:else)))

(fn ConstructionScript
  (|CallParentFunction))

(fn Lookat
  (bind _return_success (Default|InventoryList (Actor|GetComponentbyClass (Game|GetPlayerCharacter 0) "/Game/MyStuff/Final_Project/PIckupItems/Data_As/Inventory/BP_Inventory_System.BP_Inventory_System_C") (Variables|Default|Getitem) 1))
  (if _return_success
    (return "Place" (Variables|/Game/MyStuff/Final_Project/PIckupItems/Data_As/DA_Item.DA_Item_C|GetName (Variables|Default|Getitem)))
    (else
      (return "Requires" (Variables|/Game/MyStuff/Final_Project/PIckupItems/Data_As/DA_Item.DA_Item_C|GetName (Variables|Default|Getitem))))))