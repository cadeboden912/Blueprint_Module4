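; A locked drawer in Room Level 1 that opens when the player interacts while carrying the required inventory item.
; Interaction consumes the item, shows its mesh as a key and plays a timeline that inserts then withdraws it, destroys it, then slides the drawer open on a second timeline.
; Look At checks the inventory to supply the prompt verb and item name.
; Lock, unlock and key-trigger hooks are unimplemented.
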(event OnTriggered(KeyTrigger)
  (params (IsTriggered :type Boolean)))

(event Custom|Keyremove
  (bind _newtrack_0 (Timeline|KeyOpen Reverse)
    (:Update
      (Transformation|SetRelativeLocation (Variables|Default|GetKeyAnimation) (* _newtrack_0 (Variables|Default|GetKeyOpenLoca)) false false))
    (:Finished
      (CallFunction|Keyremove)
      (Utilities|FlowControl|Delay 2.0)
      (Components|DestroyComponent (Variables|Default|GetKey))
      (Utilities|FlowControl|Delay 0.5)
      ;[0.15 0.15 0.15 0.5] Still need to make key item
      (CallFunction|DrawerOpen))))

(event Custom|DrawerOpen
  (bind _newtrack_0 (Timeline|DrawerAnim Play)
    (:Update
      (Transformation|SetRelativeLocation (Variables|Default|GetScene) (* _newtrack_0 (Variables|Default|GetLocation)) false false))))

(event EventBeginPlay
  (|CallParentFunction) ; This node is disabled and will not be called.\nDrag off pins to build functionality.
)

(event Collision|EventActorBeginOverlap
  (params (OtherActor :type Actor%20Object%20Reference))
  (|CallParentFunction OtherActor) ; This node is disabled and will not be called.\nDrag off pins to build functionality.
)

(event EventTick
  (params (DeltaSeconds :type Float%20%28single-precision%29))
  (|CallParentFunction DeltaSeconds) ; This node is disabled and will not be called.\nDrag off pins to build functionality.
)

(event EventInteractwith
  (params (PlayerCharacter :type BP%20First%20Person%20Character%20Object%20Reference))
  (bind _bp_inventiry_system (Variables|/Game/FirstPerson/Blueprints/BP_FirstPersonCharacter.BP_FirstPersonCharacter_C|GetBP_Inventiry_System PlayerCharacter))
  (bind _item (Variables|Default|GetItem))
  (bind _return_success (Default|InventoryList _bp_inventiry_system (Variables|Default|GetItem) 1))
  (if _return_success
    (Default|RemovefromInventory _bp_inventiry_system _item 1)
    (Components|StaticMesh|SetStaticMesh (Variables|Default|GetKey) (Variables|/Game/MyStuff/Final_Project/PIckupItems/Data_As/DA_Item.DA_Item_C|GetStatic%20Mesh _item))
    (Components|Timeline|SetPlayRate (Variables|Default|GetKeyOpen) 3.0)
    (bind _newtrack_0 (Timeline|KeyOpen Play)
      (:Update
        (Transformation|SetRelativeLocation (Variables|Default|GetKeyAnimation) (* _newtrack_0 (Variables|Default|GetKeyOpenLoca)) false false))
      (:Finished
        (CallFunction|Keyremove)
        (Utilities|FlowControl|Delay 2.0)
        (Components|DestroyComponent (Variables|Default|GetKey))
        (Utilities|FlowControl|Delay 0.5)
        ;[0.15 0.15 0.15 0.5] Still need to make key item
        (CallFunction|DrawerOpen)))))

(fn ConstructionScript
  (|CallParentFunction))

(fn LockDoor)

(fn UnlockDoor)

(fn Lookat
  (bind _return_success (Default|InventoryList (Actor|GetComponentbyClass (Game|GetPlayerCharacter 0) "/Game/MyStuff/Final_Project/PIckupItems/Data_As/Inventory/BP_Inventory_System.BP_Inventory_System_C") (Variables|Default|GetItem) 1))
  (if _return_success
    (return "Inserted" (Variables|/Game/MyStuff/Final_Project/PIckupItems/Data_As/DA_Item.DA_Item_C|GetName (Variables|Default|GetItem)))
    (else
      (return "Requires" (Variables|/Game/MyStuff/Final_Project/PIckupItems/Data_As/DA_Item.DA_Item_C|GetName (Variables|Default|GetItem))))))