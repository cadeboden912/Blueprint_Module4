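; Password chest actor for the Level 1 room that shows a UI on interaction and animates open.
; Interactwith shows the mouse cursor, switches to UI-only input and adds a Tutorial widget to the viewport.
; OpenChest, which nothing in this graph calls, plays a timeline that slides the lid via relative location and plays a sound once.
; The lid rotation node is unconnected, and Look At returns empty prompt text.
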(event Custom|Open%20Chest
  (bind _newtrack_0 (Timeline|CHestAnim Play)
    (:Update
      (Transformation|SetRelativeLocation (Variables|Default|GetTreasureTOP_move) (* _newtrack_0 (Variables|Default|GetNew%20Location)) false false)
      (Utilities|FlowControl|DoOnce false
        (:Completed
          (Audio|PlaySound2D (Variables|Default|GetSOund) 1.0 1.0 0.0 0 0))))))

(event EventInteractwith
  (params (PlayerCharacter :type BP%20First%20Person%20Character%20Object%20Reference))
  (bind _returnvalue (Game|GetPlayerController 0))
  (Variables|/Script/Engine.PlayerController|SetbShowMouseCursor _returnvalue true)
  (Input|SetInputModeUIOnly _returnvalue 0 "DoNotLock" false)
  (bind _returnvalue_2 (UserInterface|CreateWidget "/Game/MyStuff/Final_Project/Widgets/Passcodes/Tutorial.Tutorial_C"))
  (UserInterface|Viewport|AddtoViewport _returnvalue_2 0))

(fn ConstructionScript)

(fn Lookat
  (return "" ""))