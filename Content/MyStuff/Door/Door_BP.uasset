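; Sliding door actor that the player opens by interacting, unless it is locked, and that closes when the player leaves its overlap.
; A timeline slides the Cube along DoorsDirection and reverses to close.
; A referenced Trigger's OnTriggered event unlocks or locks the door; locking also closes it.
; A point light shows red when locked and green when unlocked, and LookAt supplies the "open Door" prompt text.
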(event OnTriggered(Trigger)
  (params (IsTriggered :type Boolean))
  ;[0.15 0.1359 0.1361 0.5] When Overlapping with button
  (if IsTriggered
    (CallFunction|UnlockDoor)
    (else
      (CallFunction|LockDoor))))

(event Custom|OpenDoor
  ;[1 0 0.0426 0.009] Movement
  ;;[0.15 0.05547 0.05547 0.5] IsLock Sequence
  (if (not (Variables|Default|GetLocked))
    (bind _position (Timeline|DoorOpen Play)
      (:Update
        (Transformation|SetRelativeLocation (Variables|Default|GetCube) (* (Variables|Default|GetDoors%20Direction) _position) false false)))))

(event Custom|CloseDoor
  ;[1 0 0.0426 0.009] Movement
  (bind _position (Timeline|DoorOpen Reverse)
    (:Update
      (Transformation|SetRelativeLocation (Variables|Default|GetCube) (* (Variables|Default|GetDoors%20Direction) _position) false false))))

(event EventBeginPlay)

(event EventInteractwith
  (params (PlayerCharacter :type BP%20First%20Person%20Character%20Object%20Reference))
  (CallFunction|OpenDoor))

(event EventTick
  (params (DeltaSeconds :type Float%20%28single-precision%29)))

(event Collision|EventActorBeginOverlap
  (params (OtherActor :type Actor%20Object%20Reference))
  ;[0.15 0.15 0.15 0.5] WHen Overlapping with Door
)

(event Collision|EventActorEndOverlap
  (params (OtherActor :type Actor%20Object%20Reference))
  ;[0.15 0.15 0.15 0.5] WHen Overlapping with Door
  (if (== OtherActor (Game|GetPlayerCharacter 0))
    (CallFunction|CloseDoor)))

(fn ConstructionScript
  (Rendering|Components|Light|SetLightColor (Variables|Default|GetPointLight) (Math|Color|SelectColor "(R=1.000000,G=0.000000,B=0.000000,A=1.000000)" "(R=0.234243,G=1.000000,B=0.000000,A=1.000000)" (Variables|Default|GetLocked)) true))

(fn UnlockDoor
  (bind _output_get (Variables|Default|SetLocked false))
  ;[0.15 0.15 0.15 0.5] Color Change
  (Rendering|Components|Light|SetLightColor (Variables|Default|GetPointLight) (Math|Color|SelectColor "(R=1.000000,G=0.000000,B=0.000000,A=1.000000)" "(R=0.234243,G=1.000000,B=0.000000,A=1.000000)" _output_get) true))

(fn LockDoor
  (bind _output_get (Variables|Default|SetLocked true))
  ;[0.15 0.15 0.15 0.5] Color Change
  (Rendering|Components|Light|SetLightColor (Variables|Default|GetPointLight) (Math|Color|SelectColor "(R=1.000000,G=0.000000,B=0.000000,A=1.000000)" "(R=0.234243,G=1.000000,B=0.000000,A=1.000000)" _output_get) true)
  ;[0.15 0.15 0.15 0.5] Making Door Close When Locked
  (CallFunction|CloseDoor))

(fn Lookat
  (return "open" "Door"))